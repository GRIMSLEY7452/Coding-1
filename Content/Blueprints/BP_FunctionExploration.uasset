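; BP_FunctionExploration is a practice Blueprint that demonstrates custom events and functions through colored debug printing.
; On BeginPlay it passes each entry in Names to the Say event twice, first in magenta, then colored by GetColorByLength.
; Say treats magenta as a signal for a random color, while GetColorByLength shades from black to white by string length.
; AddTwoNumbers returns a sum with a sign-based color but is never called here.
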(event Custom|Say
  (params (InString :type String) (TextColor :type Linear%20Color%20Structure :default "(R=1.000000,G=0.000000,B=1.000000,A=1.000000)"))
  (if (== TextColor "(R=1.000000,G=0.000000,B=1.000000,A=1.000000)")
    (Development|PrintString InString true true (Utilities|Struct|MakeLinearColor (Math|Random|RandomFloat) (Math|Random|RandomFloat) (Math|Random|RandomFloat) 1.0))
    (else
      (Development|PrintString InString true true TextColor))))

(event EventBeginPlay
  (bind _names (Variables|Default|GetNames))
  (Development|PrintString "Exploring Functions")
  (for _array_element _names
    (CallFunction|Say _array_element "(R=1.000000,G=0.000000,B=1.000000,A=1.000000)"))
  (for _array_element_2 _names
    (bind _output (CallFunction|GetColorbyLength _array_element_2))
    (CallFunction|Say _array_element_2 _output)))

(fn ConstructionScript)

(fn GetColorbyLength
  (params (Input :type String))
  (bind _returnvalue (Utilities|String|Len Input))
  (bind _returnvalue_2 (- _returnvalue 5))
  (bind _returnvalue_3 (* _returnvalue_2 0.2))
  (if (<= _returnvalue 5) ; If less than 5, color = black
    (LocalVariables|SetOutputColor "")
    (elif (>= _returnvalue 10)
      (LocalVariables|SetOutputColor "(R=1.000000,G=1.000000,B=1.000000,A=1.000000)")
      (else
        (LocalVariables|SetOutputColor (Utilities|Struct|MakeLinearColor _returnvalue_3 _returnvalue_3 _returnvalue_3 1.0)) ; Set to range of colors
      )))
  (return (LocalVariables|GetOutputColor)))

(fn AddTwoNumbers
  (params (FirstNumber :type Integer) (SecondNumber :type Integer))
  (bind _returnvalue (+ FirstNumber SecondNumber))
  (if (>= _returnvalue 0)
    (LocalVariables|SetOutputColor "(R=0.000000,G=1.000000,B=0.000000,A=1.000000)")
    (else
      (LocalVariables|SetOutputColor "(R=1.000000,G=0.000000,B=0.000000,A=1.000000)")))
  (return _returnvalue (LocalVariables|GetOutputColor)))